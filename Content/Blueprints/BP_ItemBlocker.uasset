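; BP_ItemBlocker is a blocker with a Box collider that switches off while the player's camera is on the cabinet plane.
; On BeginPlay it binds to the Chemicode pawn's OnCamPlaneChanged event.
; Each change compares the new plane to the game mode's cabinet plane, disabling Box collision on a match and otherwise restoring query and physics collision.
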(event `self.ReceiveBeginPlay`
  (add `ChemicodePawn.OnCamPlaneChanged` (`ChemicodeStatics.GetChemicodePawn`) (delegate `OnCamPlaneChanged`)))

(event `OnCamPlaneChanged`
  (params (NewCamPlane :type "CameraPlane Object Reference"))
  (if (== NewCamPlane (`ChemicodeGameMode.GetCabinetCamPlane` (`ChemicodeStatics.GetChemicodeGameMode`)))
    (`PrimitiveComponent.SetCollisionEnabled` (`self.Box`) "NoCollision")
    (else
      (`PrimitiveComponent.SetCollisionEnabled` (`self.Box`) "QueryAndPhysics"))))

(fn `UserConstructionScript`)