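; BP_BunsenBurner is a Bunsen burner whose flame effect reflects its collar state and gas supply.
; On each state update it destroys the current flame and, if it has gas, attaches a safe, half or roaring Niagara flame at the mesh's Flame socket.
; Alt interaction spawns a connection preview effect at the Opening socket, moves its end point with the interaction position, and destroys it when the interaction ends.
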(event `self.OnStateUpdated`
  (params (NewState :type "EBunsenBurnerState Enum" :default "BBSCollarClosed"))
  (bind _mainmesh (`self.MainMesh`))
  (bind _flameparticle (`self.FlameParticle`))
  (bind _flameparticle_2 (`self.FlameParticle`))
  (if (`self.HasGas`)
    (if (`KismetSystemLibrary.IsValid` _flameparticle_2)
      (`ActorComponent.K2_DestroyComponent` _flameparticle_2))
    (switch `EBunsenBurnerState` NewState
      (:`BBSCollarClosed`
        (bind _returnvalue (`NiagaraFunctionLibrary.SpawnSystemAttached` "/Game/Particles/NS_SafeFlame.NS_SafeFlame" _mainmesh "Flame" (0.0 0.0 0.0) (struct) "KeepRelativeOffset"))
        (set `self.FlameParticle` _returnvalue))
      (:`BBSCollarHalfOpen`
        (bind _returnvalue_2 (`NiagaraFunctionLibrary.SpawnSystemAttached` "/Game/Particles/NS_HalfFlame.NS_HalfFlame" _mainmesh "Flame" (0.0 0.0 0.0) (struct) "KeepRelativeOffset"))
        (set `self.FlameParticle` _returnvalue_2))
      (:`BBSCollarFullyOpen`
        (bind _returnvalue_3 (`NiagaraFunctionLibrary.SpawnSystemAttached` "/Game/Particles/NS_RoaringFlame.NS_RoaringFlame" _mainmesh "Flame" (0.0 0.0 0.0) (struct) "KeepRelativeOffset"))
        (set `self.FlameParticle` _returnvalue_3)))
    (elif (`KismetSystemLibrary.IsValid` _flameparticle)
      (`ActorComponent.K2_DestroyComponent` _flameparticle))))

(event `self.UpdateAltInteractionPosition`
  (params (EndPosition :type "Vector Structure"))
  (`NiagaraComponent.SetVariableVec3` (`self.ConnectionParticle`) "EndLocation" (+ EndPosition (0.0 0.0 10.0))))

(event `self.AltInteractionBegin`
  (bind _returnvalue (`NiagaraFunctionLibrary.SpawnSystemAtLocation` "/Game/Particles/NS_ConnectionPreview.NS_ConnectionPreview" (`SceneComponent.GetSocketLocation` (`self.MainMesh`) "Opening") (struct) (1.0 1.0 1.0) false))
  (set `self.ConnectionParticle` _returnvalue))

(event `self.AltInteractionEnd`
  (`ActorComponent.K2_DestroyComponent` (`self.ConnectionParticle`)))

(fn `UserConstructionScript`)