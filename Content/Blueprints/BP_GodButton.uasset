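; BP_GodButton stages the dramatic submission of the pedestal's container for the current Chemicode assignment.
; DoSubmission starts choir audio, disables interaction, blends to an animation camera and plays a timeline that sets Speed.
; Tick uses Speed to drive post-process intensity, spin and lift the container, and reveal submission text.
; On finish, the container resets and the assignment check triggers either completion UI with confetti or failure UI with a buzzer.
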(event `self.DoSubmission`
  (bind _returnvalue (`ChemicodeStatics.GetChemicodePawn`))
  (bind _returnvalue_2 (`GameplayStatics.SpawnSound2D` "/Game/Sound/S_HolyChoir_Cue.S_HolyChoir_Cue" 1.0 1.0 0.0 null))
  (set `self.HolyChoir` _returnvalue_2)
  (set `self.InitialPosition` (`self.K2_GetActorLocation` (`SubmissionPedestal.Container` (`self.Pedestal`))))
  (`ChemicodePawn.DisableInteraction` _returnvalue)
  (`ChemicodePawn.HighlightItem` _returnvalue null)
  (`PlayerController.SetViewTargetWithBlend` (`GameplayStatics.GetPlayerController` 0) (`self.AnimCamera`) 4.0 "VTBlend_Linear" 0.0 false)
  (bind (_direction _progress) (`Timeline|Anim` :!via `PlayFromStart`)
    (:`Update`
      (set `self.Speed` _progress))
    (:`Finished`
      (set `self.Speed` 0.0)
      (`self.K2_SetActorLocation` (`SubmissionPedestal.Container` (`self.Pedestal`)) (`self.InitialPosition`) false false)
      (`ChemicodePawn.SetCamPlane` (`ChemicodeStatics.GetChemicodePawn`) (`ChemicodeGameMode.GetSubmissionCamPlane` (`ChemicodeStatics.GetChemicodeGameMode`)) 0.75)
      (`Widget.RemoveFromParent` (`self.SubmissionText`))
      (set `self.SubmissionText` null)
      (bind (_message _returnvalue_3) (`Assignment.IsCompleted` (`ChemicodeStatics.GetCurrentAssignment`) (`SubmissionPedestal.Container` (`self.Pedestal`))))
      (if _returnvalue_3
        (bind _returnvalue_4 (`|CreateWidget` "/Game/UI/W_AssignmentCompletion.W_AssignmentCompletion_C"))
        (`UserWidget.AddToViewport` _returnvalue_4 0)
        (`GameplayStatics.SpawnEmitterAtLocation` "/Game/Particles/Confetti/PS_Confetti.PS_Confetti" (`self.K2_GetActorLocation` (`SubmissionPedestal.Container` (`self.Pedestal`))) (struct))
        (`AudioComponent.Stop` (`self.HolyChoir`))
        (`GameplayStatics.PlaySound2D` "/Game/Sound/S_Confetti.S_Confetti" 1.0 1.0 0.0 null null)
        (else
          (bind _returnvalue_5 (`|CreateWidget` "/Game/UI/W_AssignmentFailure.W_AssignmentFailure_C" null (`SubmissionPedestal.Container` (`self.Pedestal`)) _message))
          (`UserWidget.AddToViewport` _returnvalue_5 0)
          (`AudioComponent.Stop` (`self.HolyChoir`))
          (`GameplayStatics.PlaySound2D` "/Game/Sound/S_Buzzer_Cue.S_Buzzer_Cue" 1.0 1.0 0.0 null null))))))

(event `self.ReceiveTick`
  (params (DeltaSeconds :type "Float (single-precision)"))
  (bind _container (`SubmissionPedestal.Container` (`self.Pedestal`)))
  (`/Engine/EditorBlueprintResources/StandardMacros.IsValid` (`SubmissionPedestal.Container` (`self.Pedestal`))
    (:`Is Valid`
      (set `PostProcessVolume.Settings` (make `PostProcessSettings` :`BloomIntensity` (* (`self.Speed`) 250.0)) (`self.PP`))
      (if (> (`self.Speed`) 0.0)
        (`self.K2_AddActorLocalRotation` _container (`KismetMathLibrary.MakeRotator` 0.0 0.0 (* (`self.Speed`) (`GameplayStatics.GetWorldDeltaSeconds`) 360.0)) false false)
        (`self.K2_SetActorLocation` _container (+ (`self.InitialPosition`) (`KismetMathLibrary.MakeVector` 0.0 0.0 (* (`self.Speed`) 70.0))) false false)
        (`/Engine/EditorBlueprintResources/StandardMacros.IsValid` (`self.SubmissionText`)
          (:`Is Not Valid`
            (if (>= (`self.Speed`) 3.0)
              (bind _returnvalue (`|CreateWidget` "/Game/UI/W_SubmissionText.W_SubmissionText_C"))
              (bind _output_get (set `self.SubmissionText` _returnvalue))
              (`UserWidget.AddToViewport` _output_get 0))))))))

(fn `UserConstructionScript`)