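; BP_ZincItem is a zinc resource item that can be oxidised by using it with another item.
; On UsewithItem it switches on its resource state: when usable and given oxygen, it shows a success notification and changes its resource to zinc oxide.
; When it still has a lid, it instead shows a notification explaining how to remove it.
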(event `self.UseWithItem`
  (params (Item :type "ResourceItem Object Reference"))
  (switch `EResourceState` (`self.ResourceState`)
    (:`Usable`
      (if (== (`ResourceItem.Resource` Item) "/Game/Resources/Data/RES_Oxygen.RES_Oxygen")
        (`ChemicodeGameMode.AddNotification` (`ChemicodeStatics.GetChemicodeGameMode`) (make `Notification` "Oxidised the zinc!" "ez" 3.0 "Success"))
        (`self.SetResource` "/Game/Resources/Data/RES_ZincOxide.RES_ZincOxide")))
    (:`HasLid`
      (`ChemicodeGameMode.AddNotification` (`ChemicodeStatics.GetChemicodeGameMode`) (make `Notification` "Take the lid off first" "To take off the lid, press E while holding the container" 3.0)))))

(fn `UserConstructionScript`
  (`parent.UserConstructionScript`))