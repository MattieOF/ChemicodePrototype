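; BP_TestTube is a test tube container item that runs simple chemical reactions on its contents.
; On each fire tick, sulfur is transferred to a valid connected tube as scaled-down sulphur dioxide; otherwise contents are removed by their "Burn Rate" property and delta time.
; When it receives sulphur dioxide, it replaces hydrogen peroxide with sulfuric acid, so two linked tubes form an acid production chain.
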(event `self.OnFireTick`
  (params (Source :type "ChemicodeObject Object Reference") (DeltaTime :type "Float (single-precision)"))
  (bind _connectedtube (`self.ConnectedTube`))
  (for _array_element (`self.Contents`)
    (bind _data (`ResourceInstance.Data` _array_element))
    (if (and (== _data "/Game/Resources/Data/RES_Sulfur.RES_Sulfur") (`KismetSystemLibrary.IsValid` _connectedtube))
      (`ResourceTube.TransferResourceAs` _connectedtube self "/Game/Resources/Data/RES_Sulfur.RES_Sulfur" "/Game/Resources/Data/RES_SulphurDioxide.RES_SulphurDioxide" (make `ResourceMeasurement` "MULitres" 50000) 0.2 true DeltaTime)
      (else
        (`self.RemoveResource` _data (make `ResourceMeasurement` "MULitres" (`KismetMathLibrary.Conv_DoubleToInt64` (* (`.ReturnValue` (`ResourceInstance.GetDecimalProperty` _array_element "Burn Rate" 0.0)) DeltaTime))))))))

(fn `OnReceiveResource`
  (params (Resource :type "ResourceData Object Reference") (Amount :type "ResourceMeasurement Structure"))
  (returns (ReturnValue :type Boolean))
  (if (<= (`.Value` (break `ResourceMeasurement` Amount)) 0)
    (return false)
    (elif (== Resource "/Game/Resources/Data/RES_SulphurDioxide.RES_SulphurDioxide")
      (bind _returnvalue (`self.ReplaceResource` "/Game/Resources/Data/RES_HydrogenPeroxide.RES_HydrogenPeroxide" "/Game/Resources/Data/RES_SulfuricAcid.RES_SulfuricAcid" Amount))
      (return _returnvalue)
      (else
        (return false)))))

(fn `UserConstructionScript`)